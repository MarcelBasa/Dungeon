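; BP_FireWall_Bolt is a bolt actor that damages the player on contact, using the damage value of the BP_FireWall that owns it.
; Its Box hit event checks for the first player character, casts the owner to BP_FireWall and applies that Damage value.
; The bolt then destroys itself, as it does on hitting anything else, but a failed owner cast on a player hit leaves it alive.
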(event OnComponentHit(Box)
  (params (HitComponent :type Primitive%20Component%20Object%20Reference) (OtherActor :type Actor%20Object%20Reference) (OtherComp :type Primitive%20Component%20Object%20Reference) (NormalImpulse :type Vector :default "0, 0, 0") (Hit :type Hit%20Result%20Structure%20%28by%20ref%29))
  (bind _returnvalue (Game|GetPlayerCharacter 0))
  (bind _self self)
  (if (== OtherActor _returnvalue)
    (bind _asbp_fire_wall (Utilities|Casting|CastToBP_FireWall (Components|GetOwner)))
    (Game|Damage|ApplyDamage _returnvalue (Variables|/Script/Dungeon.FireWall|GetDamage _asbp_fire_wall) (Game|GetInstigatorController _self) _self))
  (Actor|DestroyActor))

(event EventBeginPlay
  (|CallParentFunction) ; This node is disabled and will not be called.\nDrag off pins to build functionality.
)

(fn ConstructionScript
  (|CallParentFunction))