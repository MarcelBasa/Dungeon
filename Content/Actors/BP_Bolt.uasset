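; BP_Bolt is a short-lived bolt actor that acts as an enemy attack against the player.
; On a box hit against the player character, it applies damage using the amount and damage type of its owning Enemy, which is credited as causer.
; It destroys itself on any hit or after a brief lifetime, and spawns a small explosion particle effect whenever it is destroyed.
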(event OnComponentHit(Box)
  (params (HitComponent :type Primitive%20Component%20Object%20Reference) (OtherActor :type Actor%20Object%20Reference) (OtherComp :type Primitive%20Component%20Object%20Reference) (NormalImpulse :type Vector :default "0, 0, 0") (Hit :type Hit%20Result%20Structure%20%28by%20ref%29))
  (bind _returnvalue (Game|GetPlayerCharacter 0))
  (if (== OtherActor _returnvalue)
    (bind _asenemy (Utilities|Casting|CastToEnemy (Components|GetOwner))
      (:then
        (Game|Damage|ApplyDamage _returnvalue (Variables|/Script/Dungeon.Enemy|GetEnemyDamage _asenemy) (Game|GetInstigatorController _asenemy) _asenemy (Variables|/Script/Dungeon.Enemy|GetEnemyDamageType _asenemy)))
      (:CastFailed
        _)))
  (Actor|DestroyActor))

(event EventBeginPlay
  (Utilities|FlowControl|Delay 2.0)
  (Actor|DestroyActor))

(event EventDestroyed
  (Effects|SpawnEmitteratLocation "/Game/Assets/Particles/P_ky_explosion_playerBolt.P_ky_explosion_playerBolt" (Transformation|GetActorLocation) "0, 0, 0" "0.200000,0.200000,0.200000"))

(fn ConstructionScript)